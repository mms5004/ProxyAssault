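; BP_CameraPawn is a player camera pawn that holds little active Blueprint logic.
; StopEnableCamera toggles the MouseCanMove flag, while zoom, scroll, height and speed variables appear only as unconnected nodes.
; HeightTestBP is empty at runtime, with a disconnected downward trace that would lerp actor height toward the ground.
; DebugActorForward draws a short arrow along the root's forward vector.
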(event EventStopEnableCamera
  (params (Enable :type Boolean))
  (Variables|Default|SetMouseCanMove Enable))

(fn ConstructionScript)

(fn HeightTestBP)

(fn DebugActorForward
  (bind _rootscene (Variables|Default|GetRootScene))
  (bind _returnvalue (Transformation|GetWorldLocation _rootscene))
  (Rendering|Debug|DrawDebugArrow _returnvalue (+ _returnvalue (* (Math|Vector|GetForwardVector _rootscene) 2e+02)) 1e+01 "(R=0.780506,G=0.048201,B=0.048201,A=1.000000)" 0.4 1.0))