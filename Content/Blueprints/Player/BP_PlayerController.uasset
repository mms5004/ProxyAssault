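; Player controller for a unit-command game that stores the player's team, creates the HUD and adds unit widgets to it.
; Right-click traces under the cursor and sends a move message to each HUD-selected unit with its index and formation data.
; Square formation passes square-root-based grid sizes, while the other formations share one path passing the formation type.
; It can also possess a given unit, falling back to the default camera pawn.
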(event Input|EnhancedActionEvents|EnhancedInputActionIA_RightClick
  (params (ActionValue :type Boolean) (ElapsedSeconds :type Float%20%28double-precision%29) (TriggeredSeconds :type Float%20%28double-precision%29) (InputAction :type Input%20Action%20Object%20Reference :default "/Game/Blueprints/Player/Inputs/IA_RightClick.IA_RightClick"))
  ;[0.15 0.15 0.15 0.5] Send target to selected AI
  ; To refactor into camera pawn
  (:Started
    (Variables|Default|SetMoveLocation (.Location (Collision|BreakHitResult (.HitResult (Game|Player|GetHitResultUnderCursorbyChannel "TraceTypeQuery1" true)))))
    (bind _units (Class|BIRTS|GrabSelectedUnit(Message) (HUD|GetHUD)))
    (switch Utilities|FlowControl|Switch|SwitchonE_Formation (Variables|Default|GetFormation%20Type)
      (:NewEnumerator0
        (for (_array_element _array_index) _units
          (Class|BIRTS|UnitMove(Message) _array_element (Variables|Default|GetMoveLocation) _array_index (Utilities|Array|Length _units) "NewEnumerator0" (Math|Float|Floor (Math|Float|Sqrt (Math|Conversions|ToFloat(Integer) (Utilities|Array|Length _units)))) (* (Math|Float|Floor (Math|Float|Sqrt (Math|Conversions|ToFloat(Integer) (Utilities|Array|Length _units)))) (Math|Float|Floor (Math|Float|Sqrt (Math|Conversions|ToFloat(Integer) (Utilities|Array|Length _units))))))))
      (:NewEnumerator1
        (for (_array_element_2 _array_index_2) _units :!label _label
          (Class|BIRTS|UnitMove(Message) _array_element_2 (Variables|Default|GetMoveLocation) _array_index_2 (Utilities|Array|Length _units) (Variables|Default|GetFormation%20Type) 0 0.0)))
      (:NewEnumerator2
        (goto _label))
      (:NewEnumerator3
        (goto _label))
      (:NewEnumerator4
        (goto _label))
      (:NewEnumerator5
        (goto _label)))))

(event EventBeginPlay
  (|CallParentFunction)
  (Variables|/Script/Engine.PlayerController|SetbShowMouseCursor self true)
  (Utilities|IsValid (Variables|Default|GetPlayerHud)
    (:Is%20Not%20Valid
      (bind _returnvalue (UserInterface|CreateWidget "/Game/Blueprints/UI/WB_PlayerHUD.WB_PlayerHUD_C"))
      (Variables|Default|SetPlayerHud _returnvalue)
      (UserInterface|Viewport|AddtoViewport _returnvalue 0))))

(event EventSetUnitinHud
  (params (UnitWidget :type User%20Widget%20Object%20Reference))
  (Widget|Panel|AddChild (Variables|/Game/Blueprints/UI/WB_PlayerHUD.WB_PlayerHUD_C|GetUnits (Variables|Default|GetPlayerHud)) UnitWidget))

(event EventPlayerStart
  (params (StartActor :type Actor%20Object%20Reference) (Team :type Integer) (TeamColor :type Linear%20Color%20Structure))
  (Variables|Default|SetTeamNumber Team))

(fn ConstructionScript)

(fn GetTeam
  (return 0))

(fn GrabSelectedUnit
  (return 0))

(fn IsinSameTeam
  (params (UnitTeam :type Integer))
  (return (== UnitTeam (Variables|Default|GetTeamNumber))))

(fn SwitchUnitPlayed
  (params (UnitToPlay :type Pawn%20Object%20Reference))
  (Pawn|UnPossess)
  (Utilities|IsValid UnitToPlay
    (:Is%20Valid
      (Pawn|Possess UnitToPlay))
    (:Is%20Not%20Valid
      (Pawn|Possess (Variables|Default|GetDefaultCameraPawn)))))