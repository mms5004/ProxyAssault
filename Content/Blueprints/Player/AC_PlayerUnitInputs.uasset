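; Player input component that turns Enhanced Input actions into movement, look and run control for its owning character.
; Movement input follows control yaw, with X driving forward and Y right, while look feeds controller pitch and yaw.
; Shift raises max walk speed to RunSpeed if the character can jump, and restores WalkSpeed on release.
; The left-click action is bound but has no logic.
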(event Input|EnhancedActionEvents|EnhancedInputActionIA_Movement
  (params (ActionValue :type Vector%202D%20Structure) (ElapsedSeconds :type Float%20%28double-precision%29) (TriggeredSeconds :type Float%20%28double-precision%29) (InputAction :type Input%20Action%20Object%20Reference :default "/Game/Blueprints/Player/Inputs/IA_Movement.IA_Movement"))
  (bind _owner (Variables|Components|GetOwner))
  (bind _returnvalue (Pawn|GetControlRotation _owner :!class /Script/Engine.Pawn))
  (Pawn|Input|AddMovementInput (Variables|Components|GetOwner) (+ (* (.x ActionValue) (Math|Vector|GetForwardVector (Math|Rotator|MakeRotator 0.0 0.0 (.yaw (Pawn|GetControlRotation _owner :!class /Script/Engine.Pawn))))) (* (.y ActionValue) (Math|Vector|GetRightVector (Math|Rotator|MakeRotator (.roll _returnvalue) 0.0 (.yaw _returnvalue))))) 1.0 false))

(event Input|EnhancedActionEvents|EnhancedInputActionIA_Look
  (params (ActionValue :type Vector%202D%20Structure) (ElapsedSeconds :type Float%20%28double-precision%29) (TriggeredSeconds :type Float%20%28double-precision%29) (InputAction :type Input%20Action%20Object%20Reference :default "/Game/Blueprints/Player/Inputs/IA_Look.IA_Look"))
  (bind _owner (Variables|Components|GetOwner))
  (Pawn|Input|AddControllerPitchInput _owner (.x ActionValue))
  (Pawn|Input|AddControllerYawInput _owner (.y ActionValue)))

(event Input|EnhancedActionEvents|EnhancedInputActionIA_Shift
  (params (ActionValue :type Boolean) (ElapsedSeconds :type Float%20%28double-precision%29) (TriggeredSeconds :type Float%20%28double-precision%29) (InputAction :type Input%20Action%20Object%20Reference :default "/Game/Blueprints/Player/Inputs/IA_Shift.IA_Shift"))
  (bind _owner (Variables|Components|GetOwner))
  (bind _charactermovement (Variables|/Script/Engine.Character|GetCharacterMovement _owner))
  (:Started
    (if (Character|CanJump (Variables|Components|GetOwner))
      (Variables|/Script/Engine.CharacterMovementComponent|SetMaxWalkSpeed _charactermovement (Variables|Default|GetRunSpeed))))
  (:Completed
    (Variables|/Script/Engine.CharacterMovementComponent|SetMaxWalkSpeed _charactermovement (Variables|Default|GetWalkSpeed))))

(event Input|EnhancedActionEvents|EnhancedInputActionIA_LeftClick
  (params (ActionValue :type Boolean) (ElapsedSeconds :type Float%20%28double-precision%29) (TriggeredSeconds :type Float%20%28double-precision%29) (InputAction :type Input%20Action%20Object%20Reference :default "/Game/Blueprints/Player/Inputs/IA_LeftClick.IA_LeftClick")))