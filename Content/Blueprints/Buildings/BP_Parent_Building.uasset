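; Parent Blueprint for RTS-style buildings that can be selected and produce units for their team.
; BeginPlay creates the building panel and action buttons, and tints the mesh through a dynamic material's TeamColor parameter.
; Selection toggles the highlight and panel and messages the player pawn's camera.
; A capped queue mirrored by removable UI buttons feeds a timer-driven counter, which spawns each unit at SpawnPoint with the building's team number and color.
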(event Custom|ProcessProduction
  ;[0.1781 1 0.2742] Counter + create new unit
  (if (and (Variables|Producing|GetIsProducing?) (< (Variables|Producing|GetProductionCounter) (Variables|Producing|GetProduction%20Time%20Needed)))
    (Variables|Producing|SetProductionCounter (+ (Variables|Producing|GetProductionCounter) (Variables|Producing|GetProductionUpdateTime)))
    (elif (Variables|Producing|GetIsProducing?)
      (Variables|Producing|SetIsProducing? false)
      (Game|SpawnActorfromClass (Utilities|Array|Get(acopy) (Variables|Producing|GetUnitProductionQueue)) (Transformation|GetWorldTransform (Variables|Default|GetSpawnPoint)) "AdjustIfPossibleButAlwaysSpawn" "SelectDefaultAtRuntime" 0 (Variables|Default|GetTeamNumber) (Variables|Default|GetTeamColor) 0)
      (CallFunction|RemoveUnit 0 true))))

(event Custom|FirstProductUpdate
  ;[0.464 0.1676 1] Display Current unit
  (Class|Image|SetBrush (Variables|/Game/Blueprints/UI/WB_Buildings.WB_Buildings_C|GetCurrentUnitProduction (Variables|Producing|GetBuildingSeletedWidget)) (Utilities|Struct|MakeSlateBrush "(SpecifiedColor=(R=1.000000,G=1.000000,B=1.000000,A=1.000000),ColorUseRule=UseColor_Specified)" "Image" "NoTile" "NoMirror" "(X=32.000000,Y=32.000000)" "(Left=0.000000,Top=0.000000,Right=0.000000,Bottom=0.000000)" (.UnitImage (Utilities|GetClassDefaults (Utilities|Array|Get(acopy) (Variables|Producing|GetUnitProductionQueue)))) "(CornerRadii=(X=0.000000,Y=0.000000,Z=0.000000,W=0.000000),Color=(SpecifiedColor=(R=0.000000,G=0.000000,B=0.000000,A=0.000000),ColorUseRule=UseColor_Specified),Width=0.000000,RoundingType=HalfHeightRadius,bUseBrushTransparency=False)")))

(event Custom|NextUnitProduct
  ;[1 0.1769 0.7414] Next Unit
  (if (> (Utilities|Array|Length (Variables|Producing|GetUnitProductionQueue)) 0)
    (CallFunction|FirstProductUpdate)
    (Variables|Producing|SetIsProducing? true)
    (Variables|Producing|SetProductionCounter 0.0)
    (Variables|Producing|SetProduction%20Time%20Needed (.ProductionTime (Utilities|GetClassDefaults (Utilities|Array|Get(acopy) (Variables|Producing|GetUnitProductionQueue)))))
    (Utilities|Time|SetTimerbyEvent (delegate Custom|ProcessProduction) (Variables|Producing|GetProductionUpdateTime) (Variables|Producing|GetIsProducing?))))

(event Custom|RemoveUnit
  (params (WB :type WB%20T%20Unit%20Object%20Reference) (First :type Boolean))
  (bind _unitbuttonslist (Variables|Producing|GetUnitButtonsList))
  (bind _returnvalue (Utilities|Array|FindItem _unitbuttonslist WB))
  (if (> (Utilities|Array|Length (Variables|Producing|GetUnitButtonsList)) 0)
    (if First
      ;[0.1309 1 0.1457] Next unit (delete first button)
      (Widget|RemovefromParent (Utilities|Array|Get(acopy) (Variables|Producing|GetUnitButtonsList)))
      (Utilities|Array|RemoveIndex (Variables|Producing|GetUnitButtonsList))
      (Utilities|Array|RemoveIndex (Variables|Producing|GetUnitProductionQueue))
      (CallFunction|NextUnitProduct)
      (else
        ;[1 0.2228 0.2626] Remove a button clicked
        (Utilities|Array|RemoveIndex (Variables|Producing|GetUnitProductionQueue) _returnvalue)
        (Widget|RemovefromParent (Utilities|Array|Get(acopy) _unitbuttonslist _returnvalue))
        (Utilities|Array|RemoveIndex (Variables|Producing|GetUnitButtonsList) _returnvalue)
        (CallFunction|NextUnitProduct)))
    (else
      ;[0.3488 0.1094 1] When the last unit is produced it unlist it
      (if (> (Utilities|Array|Length (Variables|Producing|GetUnitProductionQueue)) 0)
        (Utilities|Array|Clear (Variables|Producing|GetUnitProductionQueue))))))

(event Custom|AddUnitList
  (bind _unitproductionqueue (Variables|Producing|GetUnitProductionQueue))
  ;[0.4218 0.2155 1] Add first Unit
  (if (> (Utilities|Array|Length (Variables|Producing|GetUnitProductionQueue)) 1)
    ;[0.9198 1 0] Add a new button when adding an unit
    (bind _returnvalue (UserInterface|CreateWidget (Variables|Producing|GetNewUnitButton)))
    (Widget|Transform|SetRenderScale _returnvalue "(X=0.800000,Y=0.800000)")
    (Variables|/Game/Blueprints/UI/Units/WB_T_Unit.WB_T_Unit_C|SetIsListed _returnvalue true)
    (Utilities|Array|Add (Variables|Producing|GetUnitButtonsList) _returnvalue)
    (Variables|/Game/Blueprints/UI/Units/WB_T_Unit.WB_T_Unit_C|SetBuildingreference _returnvalue self)
    (Class|Image|SetBrush (Variables|/Game/Blueprints/UI/Units/WB_T_Unit.WB_T_Unit_C|GetImage _returnvalue) (Utilities|Struct|MakeSlateBrush "(SpecifiedColor=(R=1.000000,G=1.000000,B=1.000000,A=1.000000),ColorUseRule=UseColor_Specified)" "Image" "NoTile" "NoMirror" "(X=32.000000,Y=32.000000)" "(Left=0.000000,Top=0.000000,Right=0.000000,Bottom=0.000000)" (.UnitImage (Utilities|GetClassDefaults (Utilities|Array|Get(acopy) _unitproductionqueue (Utilities|Array|LastIndex _unitproductionqueue)))) "(CornerRadii=(X=0.000000,Y=0.000000,Z=0.000000,W=0.000000),Color=(SpecifiedColor=(R=0.000000,G=0.000000,B=0.000000,A=0.000000),ColorUseRule=UseColor_Specified),Width=0.000000,RoundingType=HalfHeightRadius,bUseBrushTransparency=False)"))
    (for _array_element (Variables|Producing|GetUnitButtonsList)
      (Class|WrapBox|AddChildtoWrapBox (Variables|/Game/Blueprints/UI/WB_Buildings.WB_Buildings_C|GetUnitList (Variables|Producing|GetBuildingSeletedWidget)) _array_element))
    (else
      (CallFunction|FirstProductUpdate))))

(event Custom|DeleteCurrentUnit
  ;[0.5579 0.4075 1] Press/delete current Unit
  (if (> (Utilities|Array|Length (Variables|Producing|GetUnitProductionQueue)) 0)
    (Utilities|Array|RemoveIndex (Variables|Producing|GetUnitProductionQueue))
    (if (> (Utilities|Array|Length (Variables|Producing|GetUnitButtonsList)) 0)
      (Widget|RemovefromParent (Utilities|Array|Get(acopy) (Variables|Producing|GetUnitButtonsList)))
      (Utilities|Array|RemoveIndex (Variables|Producing|GetUnitButtonsList))
      (CallFunction|NextUnitProduct)
      (else
        (Variables|Producing|SetIsProducing? false)))))

(event EventProduceUnit
  (params (Unit :type BP%20Parent%20Unit%20Class%20Reference) (UnitButton :type WB%20T%20Unit%20Class%20Reference))
  (if (<= (Utilities|Array|Length (Variables|Producing|GetUnitProductionQueue)) 10)
    (Variables|Producing|SetUnitBeingProduce Unit)
    (Variables|Producing|SetNewUnitButton UnitButton)
    (Utilities|Array|Add (Variables|Producing|GetUnitProductionQueue) Unit)
    (CallFunction|AddUnitList)
    (if (and (> (Utilities|Array|Length (Variables|Producing|GetUnitProductionQueue)) 0) (not (Variables|Producing|GetIsProducing?)))
      (Variables|Producing|SetIsProducing? true)
      (Variables|Producing|SetProductionCounter 0.0)
      (Variables|Producing|SetProduction%20Time%20Needed (.ProductionTime (Utilities|GetClassDefaults (Utilities|Array|Get(acopy) (Variables|Producing|GetUnitProductionQueue)))))
      (Utilities|Time|SetTimerbyEvent (delegate Custom|ProcessProduction) (Variables|Producing|GetProductionUpdateTime) (Variables|Producing|GetIsProducing?)))))

(event EventDeselectThings
  (Rendering|SetVisibility (Variables|Default|GetSelection) false false)
  (Widget|RemovefromParent (Variables|Producing|GetBuildingSeletedWidget))
  (Class|BIPlayer|StopEnableCamera(Message) (Game|Player|GetPlayerPawn 0) true))

(event EventSelectThings
  (Rendering|SetVisibility (Variables|Default|GetSelection) true false)
  (UserInterface|Viewport|AddtoViewport (Variables|Producing|GetBuildingSeletedWidget) 0)
  (Class|BIPlayer|StopEnableCamera(Message) (Game|Player|GetPlayerPawn 0) false))

(event EventBeginPlay
  (Utilities|FlowControl|Sequence
    (:then_0
      (for _array_element (Variables|Default|GetUnitCanBeProduce)
        (bind _returnvalue (UserInterface|CreateWidget _array_element))
        (Utilities|Array|AddUnique (Variables|Producing|GetActionBoxButtons) _returnvalue)
        (Variables|/Game/Blueprints/UI/Units/WB_T_Unit.WB_T_Unit_C|SetBuildingreference _returnvalue self)))
    (:then_1
      (Utilities|FlowControl|Sequence
        (:then_0
          ;[1 1 1] Create widget
          (bind _returnvalue_2 (UserInterface|CreateWidget "/Game/Blueprints/UI/WB_Buildings.WB_Buildings_C"))
          (Variables|Producing|SetBuildingSeletedWidget _returnvalue_2)
          (Variables|/Game/Blueprints/UI/WB_Buildings.WB_Buildings_C|SetBuildingReference _returnvalue_2 self)
          (for _array_element_2 (Variables|Producing|GetActionBoxButtons)
            (Class|WrapBox|AddChildtoWrapBox (Variables|/Game/Blueprints/UI/WB_Buildings.WB_Buildings_C|GetActionBox (Variables|Producing|GetBuildingSeletedWidget)) _array_element_2)))
        (:then_1
          ;[1 1 1] Set team Color
          (bind _returnvalue_3 (Rendering|Material|CreateDynamicMaterialInstance (Rendering|Material|GetMaterial (Variables|Default|GetBuildingMesh) 0) "None" "None" :!class /Script/Engine.KismetMaterialLibrary))
          (Rendering|Material|SetVectorParameterValue _returnvalue_3 "TeamColor" (Variables|Default|GetTeamColor) :!class /Script/Engine.MaterialInstanceDynamic)
          (Rendering|Material|SetMaterial (Variables|Default|GetBuildingMesh) 0 _returnvalue_3))))))

(fn ConstructionScript)

(fn GetTeam
  (return (Variables|Default|GetTeamNumber)))

(fn GrabSelectedUnit
  (return 0))

(fn IsinSameTeam
  (params (UnitTeam :type Integer))
  (return false))