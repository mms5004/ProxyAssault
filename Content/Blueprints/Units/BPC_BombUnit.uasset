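; BPC_BombUnit is a bomb unit Blueprint that the player moves around as a physics-driven sphere.
; Movement input applies a velocity-change impulse to the sphere, scaled by RollTorque and oriented by the player camera's yaw.
; It then caps X and Y using the full velocity vector clamped to MaxVelocity, while keeping the original Z so vertical motion is preserved.
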(event Input|EnhancedActionEvents|EnhancedInputActionIA_Movement
  (params (ActionValue :type Vector%202D%20Structure) (ElapsedSeconds :type Float%20%28double-precision%29) (TriggeredSeconds :type Float%20%28double-precision%29) (InputAction :type Input%20Action%20Object%20Reference :default "/Game/Blueprints/Player/Inputs/IA_Movement.IA_Movement"))
  (bind _returnvalue (Game|GetPlayerCameraManager 0))
  (bind _sphere (Variables|Default|GetSphere))
  (bind _maxvelocity (Variables|Default|GetMaxVelocity))
  (bind _sphere_2 (Variables|Default|GetSphere))
  (bind _returnvalue_2 (Transformation|GetComponentVelocity _sphere_2))
  (bind _returnvalue_3 (Camera|GetCameraRotation _returnvalue))
  (bind _returnvalue_4 (* -1.0 _maxvelocity))
  (bind _returnvalue_5 (Math|Vector|ClampVectorSize _returnvalue_2 _returnvalue_4 _maxvelocity))
  ;[0.09896 0.09896 0.09896 0.5435] Rolling
  (Class|PrimitiveComponent|AddVelocityChangeImpulseatLocation _sphere (+ (* (Math|Vector|GetForwardVector (Math|Rotator|MakeRotator 0.0 0.0 (.yaw _returnvalue_3))) (Variables|Default|GetRollTorque) (.x ActionValue)) (* (* (.y ActionValue) (Variables|Default|GetRollTorque)) (Math|Vector|GetRightVector (Math|Rotator|MakeRotator 0.0 0.0 (.yaw _returnvalue_3))))) (Transformation|GetWorldLocation _sphere) "None")
  (Physics|SetPhysicsLinearVelocity (Variables|Default|GetSphere) (Math|Vector|MakeVector (.x _returnvalue_5) (.y _returnvalue_5) (.z (Transformation|GetComponentVelocity (Variables|Default|GetSphere)))) false "None"))

(fn ConstructionScript)