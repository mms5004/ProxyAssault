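; Base Blueprint for selectable, team-colored units that move in group formations.
; BeginPlay creates the unit's widget and tints its mesh via a dynamic material, while selection and highlight events drive a decal and the HUD widget.
; UnitMove offsets the target by the unit's group index into square, circle, column, line or diagonal formations, all camera-oriented except circle.
; MoveToLocation then restarts AI movement toward that point.
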(event Custom|MoveToLocation
  (bind _self self)
  (bind _returnvalue (AI|GetAIController _self))
  (AI|Navigation|StopMovement _returnvalue)
  (AI|AIMoveTo _returnvalue (Variables|Default|GetTargetLocation) 0 -1.0 "Default" "Default" true false))

(event EventBeginPlay
  (Utilities|FlowControl|Sequence
    (:then_0
      (bind _returnvalue (UserInterface|CreateWidget "/Game/Blueprints/UI/Units/WB_SelectedUnit.WB_SelectedUnit_C"))
      (bind _output_get (Variables|Default|SetUnitWidget _returnvalue))
      (Variables|/Game/Blueprints/UI/Units/WB_SelectedUnit.WB_SelectedUnit_C|SetUnitReference _output_get self)
      (Appearance|SetBrushfromTexture (Variables|/Game/Blueprints/UI/Units/WB_SelectedUnit.WB_SelectedUnit_C|GetUnitImage _output_get) (Variables|Default|GetUnitImage) false))
    (:then_1
      ;[1 1 1] Set team color
      (bind _returnvalue_2 (Rendering|Material|CreateDynamicMaterialInstance (Rendering|Material|GetMaterial (Variables|Default|GetCube) 0) "None" "None" :!class /Script/Engine.KismetMaterialLibrary))
      (Rendering|Material|SetVectorParameterValue _returnvalue_2 "TeamColor" (Variables|Default|GetTeamColor) :!class /Script/Engine.MaterialInstanceDynamic)
      (Rendering|Material|SetMaterial (Variables|Default|GetCube) 0 _returnvalue_2))))

(event Collision|EventActorBeginOverlap
  (params (OtherActor :type Actor%20Object%20Reference)))

(event EventTick
  (params (DeltaSeconds :type Float%20%28single-precision%29)))

(event EventSelectThings
  (Rendering|SetVisibility (Variables|Default|GetDecal) true false)
  (Class|BIRTS|SetUnitinHud(Message) (Game|GetPlayerController 0) (Variables|Default|GetUnitWidget)))

(event EventDeselectThings
  (Rendering|SetVisibility (Variables|Default|GetDecal) false false)
  (Widget|RemovefromParent (Variables|Default|GetUnitWidget)))

(event EventUnitMove
  (params (Location :type Vector :default "0, 0, 0") (Index :type Integer) (TotalIndex :type Integer) (FormationType :type E_Formation%20Enum :default "NewEnumerator0") (SquareLength :type Integer) (SquareLast :type Float%20%28double-precision%29))
  (Variables|Default|SetIndex (Math|Conversions|ToFloat(Integer) Index))
  (Variables|Default|SetTotal%20Index (Math|Conversions|ToFloat(Integer) TotalIndex))
  (Variables|Default|SetTargetLocation Location)
  (if (> TotalIndex 1)
    (switch Utilities|FlowControl|Switch|SwitchonE_Formation FormationType
      (:NewEnumerator0
        (CallFunction|Square SquareLength SquareLast))
      (:NewEnumerator1
        (CallFunction|CircleFormation))
      (:NewEnumerator2
        (CallFunction|Column))
      (:NewEnumerator3
        (CallFunction|Line))
      (:NewEnumerator4
        (CallFunction|Diagonal false))
      (:NewEnumerator5
        (CallFunction|Diagonal true)))
    (else
      (CallFunction|MovetoLocation))))

(event EventHighlightUnit
  (Rendering|Components|Decal|SetDecalMaterial (Variables|Default|GetDecal) "/Game/Materials/M_UnitSelectDecalHighlight.M_UnitSelectDecalHighlight"))

(event EventUnHighlightUnit
  (Rendering|Components|Decal|SetDecalMaterial (Variables|Default|GetDecal) "/Game/Materials/M_UnitSelectDecal.M_UnitSelectDecal"))

(fn ConstructionScript)

(fn Square
  (params (SquareLength :type Integer) (Last :type Float%20%28double-precision%29))
  (bind _returnvalue (Math|Conversions|ToFloat(Integer) SquareLength))
  (bind _returnvalue_2 (Math|Conversions|ToFloat(Integer) SquareLength))
  (bind _distance (Variables|Default|GetDistance))
  (bind _distance_2 (Variables|Default|GetDistance))
  (bind _returnvalue_3 (* _distance_2 _returnvalue -0.25))
  (Variables|Default|SetTargetLocation (+ (Math|Vector|RotateVectorAroundAxis (Math|Vector|MakeVector (+ _returnvalue_3 (* (Math|Float|%(Float) (Variables|Default|GetIndex) _returnvalue_2) _distance)) (+ _returnvalue_3 (* _distance (Math|Float|Floor (/ (Variables|Default|GetIndex) _returnvalue_2)))) 0.0) (.yaw (Transformation|GetWorldRotation (Variables|/Script/Engine.PlayerCameraManager|GetTransformComponent (Game|GetPlayerCameraManager 0)))) "0, 0,1.000000") (Variables|Default|GetTargetLocation)))
  (CallFunction|MovetoLocation)
  (return))

(fn CircleFormation
  (Variables|Default|SetTargetLocation (+ (Variables|Default|GetTargetLocation) (* (Math|Vector|GetForwardVector (Math|Rotator|MakeRotator 0.0 0.0 (* (Variables|Default|GetIndex) (/ 3.6e+02 (Variables|Default|GetTotal%20Index))))) (Variables|Default|GetDistance))))
  (CallFunction|MovetoLocation)
  (return))

(fn Column
  (bind _distance (Variables|Default|GetDistance))
  (bind _distance_2 (Variables|Default|GetDistance))
  (bind _index (Variables|Default|GetIndex))
  (bind _total_index (Variables|Default|GetTotal%20Index))
  (bind _returnvalue (* _total_index _distance -0.5))
  (bind _returnvalue_2 (* _distance_2 _index))
  (bind _returnvalue_3 (+ _returnvalue_2 _returnvalue))
  (Variables|Default|SetTargetLocation (+ (* (Math|Vector|GetForwardVector (Variables|/Script/Engine.PlayerCameraManager|GetTransformComponent (Game|GetPlayerCameraManager 0))) (Math|Vector|MakeVector _returnvalue_3 _returnvalue_3 0.0)) (Variables|Default|GetTargetLocation)))
  (CallFunction|MovetoLocation))

(fn Line
  (bind _distance (Variables|Default|GetDistance))
  (bind _distance_2 (Variables|Default|GetDistance))
  (bind _index (Variables|Default|GetIndex))
  (bind _total_index (Variables|Default|GetTotal%20Index))
  (bind _returnvalue (* _total_index _distance -0.5))
  (bind _returnvalue_2 (* _distance_2 _index))
  (bind _returnvalue_3 (+ _returnvalue_2 _returnvalue))
  (Variables|Default|SetTargetLocation (+ (* (Math|Vector|GetRightVector (Variables|/Script/Engine.PlayerCameraManager|GetTransformComponent (Game|GetPlayerCameraManager 0))) (Math|Vector|MakeVector _returnvalue_3 _returnvalue_3 0.0)) (Variables|Default|GetTargetLocation)))
  (CallFunction|MovetoLocation))

(fn Diagonal
  (params (BiggerSmaller :type Boolean))
  (bind _returnvalue (Game|GetPlayerCameraManager 0))
  (bind _returnvalue_2 (Game|GetPlayerCameraManager 0))
  (bind _distance (Variables|Default|GetDistance))
  (bind _total_index (Variables|Default|GetTotal%20Index))
  (bind _distance_2 (Variables|Default|GetDistance))
  (bind _total_index_2 (Variables|Default|GetTotal%20Index))
  (bind _distance_3 (Variables|Default|GetDistance))
  (bind _index (Variables|Default|GetIndex))
  (bind _index_2 (Variables|Default|GetIndex))
  (bind _distance_4 (Variables|Default|GetDistance))
  (bind _returnvalue_3 (* _total_index_2 _distance -0.5))
  (bind _returnvalue_4 (* _distance_3 _index_2))
  (bind _returnvalue_5 (* _distance_4 _total_index))
  (bind _returnvalue_6 (* _index _distance_2 -0.5))
  (bind _transformcomponent (Variables|/Script/Engine.PlayerCameraManager|GetTransformComponent _returnvalue))
  (bind _transformcomponent_2 (Variables|/Script/Engine.PlayerCameraManager|GetTransformComponent _returnvalue_2))
  (bind _returnvalue_7 (+ _returnvalue_5 _returnvalue_6))
  (bind _returnvalue_8 (+ _returnvalue_4 _returnvalue_3))
  (if BiggerSmaller
    (Variables|Default|SetTargetLocation (+ (Variables|Default|GetTargetLocation) (* (Math|Vector|Normalize (+ (Math|Vector|GetForwardVector _transformcomponent_2) (Math|Vector|GetRightVector _transformcomponent_2))) (Math|Vector|MakeVector _returnvalue_8 _returnvalue_8 0.0))))
    (else
      (Variables|Default|SetTargetLocation (+ (* (Math|Vector|MakeVector _returnvalue_7 _returnvalue_7 0.0) (Math|Vector|Normalize (+ (Math|Vector|GetForwardVector _transformcomponent) (* (Math|Vector|GetRightVector _transformcomponent) -1.0)))) (Variables|Default|GetTargetLocation)))))
  (CallFunction|MovetoLocation))

(fn GetTeam
  (return (Variables|Default|GetTeamNumber)))

(fn GrabSelectedUnit
  (return 0))

(fn IsinSameTeam
  (params (UnitTeam :type Integer))
  (return false))